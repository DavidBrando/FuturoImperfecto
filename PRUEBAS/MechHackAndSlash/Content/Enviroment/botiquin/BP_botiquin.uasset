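; BP_botiquin is a first-aid kit pickup meant to heal the player's Warrior_BP character.
; A Box overlap with the player fires once, printing a debug message, spawning the P_heal emitter at the mesh, then destroying the actor after a short delay.
; No health is actually applied, as the Curacion variable is unused.
; A Timeline-driven vertical movement for the mesh exists but is disconnected and never runs.
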(event `self.ReceiveTick`
  (params (DeltaSeconds :type "Float (single-precision)")))

(event `self.Box.OnComponentBeginOverlap`
  (params (OverlappedComponent :type "PrimitiveComponent Object Reference") (OtherActor :type "Actor Object Reference") (OtherComp :type "PrimitiveComponent Object Reference") (OtherBodyIndex :type Integer) (bFromSweep :type Boolean) (SweepResult :type "HitResult Structure (by ref)"))
  (if (== OtherActor (`GameplayStatics.GetPlayerCharacter` 0))
    (cast `/Game/Jugador/Warrior_BP` OtherActor)
    (`/Engine/EditorBlueprintResources/StandardMacros.DoOnce` false
      (:`Completed`
        (`KismetSystemLibrary.PrintString` "aqui av la vida")
        (`GameplayStatics.SpawnEmitterAtLocation` "/Game/StarterContent/Particles/p_heal.p_heal" (`SceneComponent.K2_GetComponentLocation` (`self.StaticMesh`)))
        (`KismetSystemLibrary.Delay` 0.2)
        (`self.K2_DestroyActor`)))))

(fn `UserConstructionScript`)