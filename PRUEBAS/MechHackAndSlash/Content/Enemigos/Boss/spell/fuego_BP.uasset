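; Boss spell fire hazard actor that burns and damages the player character.
; After a one-second delay it swaps the PFire component for Fire and enables the Sphere's collision, then destroys itself ten seconds later.
; When a Warrior_BP begins overlapping the Sphere, it calls BurnPMessage on the player character and applies a small ranged damage amount through RecibirDamage.
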(event `self.ReceiveBeginPlay`
  (`KismetSystemLibrary.Delay` 1.0)
  (`SceneComponent.SetHiddenInGame` (`self.fire`) false false)
  (`SceneComponent.SetHiddenInGame` (`self.p_fire`) true false)
  (`PrimitiveComponent.SetCollisionEnabled` (`self.Sphere`) "QueryAndPhysics")
  (`KismetSystemLibrary.Delay` 10.0)
  (`self.K2_DestroyActor`))

(event `self.Sphere.OnComponentBeginOverlap`
  (params (OverlappedComponent :type "PrimitiveComponent Object Reference") (OtherActor :type "Actor Object Reference") (OtherComp :type "PrimitiveComponent Object Reference") (OtherBodyIndex :type Integer) (bFromSweep :type Boolean) (SweepResult :type "HitResult Structure (by ref)"))
  (bind _returnvalue (`GameplayStatics.GetPlayerCharacter` 0))
  (if (== (`GameplayStatics.GetObjectClass` OtherActor) "/Game/Jugador/Warrior_BP.Warrior_BP_C")
    (bind _aswarrior_bp (cast `/Game/Jugador/Warrior_BP` _returnvalue))
    (message `/Game/General/BPI_Debuff.Burn_P` _returnvalue)
    (`/Game/Jugador/Warrior_BP.RecibirDamage` _aswarrior_bp 4.0 5.0)))

(fn `UserConstructionScript`)