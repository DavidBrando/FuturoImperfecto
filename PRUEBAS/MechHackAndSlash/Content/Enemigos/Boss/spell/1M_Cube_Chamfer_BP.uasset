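; Boss spell projectile actor, apparently a fireball, that damages the Warrior player on contact.
; On spawn it waits briefly before enabling its sphere's collision, then destroys itself after a few seconds if still alive.
; A sphere overlap with Warrior_BP calls RecibirDamage on the player character with a damage range, spawns a fireball hit emitter and destroys the actor.
; Any other overlap also destroys it, printing a debug string.
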(event `self.ReceiveBeginPlay`
  (`KismetSystemLibrary.Delay` 0.2)
  (`PrimitiveComponent.SetCollisionEnabled` (`self.Sphere`) "QueryAndPhysics")
  (`KismetSystemLibrary.Delay` 5.0)
  (`self.K2_DestroyActor`))

(event `self.Sphere.OnComponentBeginOverlap`
  (params (OverlappedComponent :type "PrimitiveComponent Object Reference") (OtherActor :type "Actor Object Reference") (OtherComp :type "PrimitiveComponent Object Reference") (OtherBodyIndex :type Integer) (bFromSweep :type Boolean) (SweepResult :type "HitResult Structure (by ref)"))
  (if (== (`GameplayStatics.GetObjectClass` OtherActor) "/Game/Jugador/Warrior_BP.Warrior_BP_C")
    (bind _aswarrior_bp (cast `/Game/Jugador/Warrior_BP` (`GameplayStatics.GetPlayerCharacter` 0)))
    (`/Game/Jugador/Warrior_BP.RecibirDamage` _aswarrior_bp 10.0 15.0)
    (`GameplayStatics.SpawnEmitterAtLocation` "/Game/StarterContent/Particles/hitBolaDeFuego.hitBolaDeFuego" (`SceneComponent.K2_GetComponentLocation` (`self.Sphere`)))
    (`KismetSystemLibrary.Delay` 0.001)
    (`self.K2_DestroyActor`)
    (else
      (`KismetSystemLibrary.Delay` 0.001)
      (`self.K2_DestroyActor`)
      (`KismetSystemLibrary.PrintString` "MUEROME" true true (struct :`R` 1.0 :`G` 0.14596 :`B` 0.99993 :`A` 1.0)))))

(fn `UserConstructionScript`)